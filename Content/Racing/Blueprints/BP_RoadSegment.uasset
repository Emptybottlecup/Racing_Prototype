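; BP_RoadSegment is a racing road piece that builds its surface along a spline and can spawn a following segment.
; The construction script tiles spline meshes along the chosen spline, whose random pick is pinned to Spline1.
; BeginPlay moves AttachPoint near the spline's end, where SpawnNewRoad places the next segment.
; Overlapping Box destroys the segment after a delay, while overlapping Box1 opens the ThirdPersonTemplate level.
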(event OnComponentBeginOverlap(Box)
  (params (OverlappedComponent :type Primitive%20Component%20Object%20Reference) (OtherActor :type Actor%20Object%20Reference) (OtherComp :type Primitive%20Component%20Object%20Reference) (OtherBodyIndex :type Integer) (bFromSweep :type Boolean) (SweepResult :type Hit%20Result%20Structure%20%28by%20ref%29))
  (Utilities|FlowControl|Delay 5.0)
  (Actor|DestroyActor))

(event OnComponentBeginOverlap(Box1)
  (params (OverlappedComponent :type Primitive%20Component%20Object%20Reference) (OtherActor :type Actor%20Object%20Reference) (OtherComp :type Primitive%20Component%20Object%20Reference) (OtherBodyIndex :type Integer) (bFromSweep :type Boolean) (SweepResult :type Hit%20Result%20Structure%20%28by%20ref%29))
  (Game|OpenLevel(byName) "ThirdPersonTemplate"))

(event Custom|SpawnNewRoad
  (bind _returnvalue (Transformation|GetActorTransform))
  (Game|SpawnActorfromClass "BP_RoadSegment_C" (Math|Transform|MakeTransform (Transformation|GetWorldLocation (Variables|Default|GetAttachPoint)) (.rotation _returnvalue) (.scale _returnvalue)) "Undefined" "MultiplyWithRoot" 0 2e+02 0))

(event EventBeginPlay
  (bind _chosenspline (Variables|Default|GetChosenSpline))
  (bind _chosenspline_2 (Variables|Default|GetChosenSpline))
  (bind _returnvalue (Spline|GetNumberOfSplinePoints _chosenspline))
  (bind _returnvalue_2 (- _returnvalue 1))
  (bind _returnvalue_3 (Spline|GetLocationatSplinePoint _chosenspline_2 _returnvalue_2 "Local"))
  (Transformation|SetRelativeLocation (Variables|Default|GetAttachPoint) (Math|Vector|MakeVector (- (.x _returnvalue_3) 35.0) (.y _returnvalue_3) (.z _returnvalue_3)) false false))

(fn ConstructionScript
  (bind _meshsize (Variables|Default|GetMeshSize))
  (Variables|Default|SetChosenSpline (Utilities|Select :Index (Math|Random|RandomIntegerinRange 1 1) :Option%200 (Variables|Default|GetSpline2) :Option%201 (Variables|Default|GetSpline1) :Option%202 (Variables|Default|GetSpline3)))
  (for _index (range 0 (Math|Float|Truncate (/ (Spline|GetSplineLength (Variables|Default|GetChosenSpline)) (Variables|Default|GetMeshSize))))
    (if (not (> (+ (* _index _meshsize) _meshsize) (Spline|GetSplineLength (Variables|Default|GetChosenSpline))))
      (bind _returnvalue (AddComponent|AddSplineMeshComponent false))
      (SplineMesh|SetStartandEnd _returnvalue (Spline|GetLocationatDistanceAlongSpline (Variables|Default|GetChosenSpline) (* _index _meshsize) "Local") (Math|Vector|ClampVectorSize (Spline|GetTangentatDistanceAlongSpline (Variables|Default|GetChosenSpline) (* _index _meshsize) "Local") 0.0 (Variables|Default|GetMeshSize)) (Spline|GetLocationatDistanceAlongSpline (Variables|Default|GetChosenSpline) (+ (* _index _meshsize) _meshsize) "Local") (Math|Vector|ClampVectorSize (Spline|GetTangentatDistanceAlongSpline (Variables|Default|GetChosenSpline) (+ (* _index _meshsize) _meshsize) "Local") 0.0 (Variables|Default|GetMeshSize)) true :!class /Script/Engine.SplineMeshComponent))))