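; Racing game mode that builds the track at runtime from chained BP_RoadSegment actors.
; BeginPlay spawns an initial batch of segments and starts a looping timer.
; Each spawn places a scaled segment at the stored AttachPoint, then updates it from the new segment's attach component, so pieces join end to end by location.
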(event Custom|Spawn%20Road
  (bind _returnvalue (Game|SpawnActorfromClass "/Game/Racing/Blueprints/BP_RoadSegment.BP_RoadSegment_C" (Math|Transform|MakeTransform (Variables|Default|GetAttachPoint) "0, 0, 0" "15.000000,15.000000,15.000000") "Undefined" "MultiplyWithRoot" 0 2e+02 0))
  (Variables|Default|SetAttachPoint (Transformation|GetWorldLocation (Variables|/Game/Racing/Blueprints/BP_RoadSegment.BP_RoadSegment_C|GetAttachPoint _returnvalue))))

(event Custom|CustomEvent
  (for _index (range 0 10)
    (CallFunction|SpawnRoad)))

(event EventBeginPlay
  (CallFunction|CustomEvent)
  (Utilities|Time|SetTimerbyEvent (EventDispatchers|CreateEvent :!event Custom|CustomEvent) 1e+02 true))

(fn ConstructionScript)